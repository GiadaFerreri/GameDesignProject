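; Robot enemy that spots the first-person player, attacks with a laser and sends them back to a fixed point when caught.
; PawnSensing writes seen and in-range flags to the AI Blackboard, using keys suffixed with 4.
; AttackPlayer4 sphere-traces ahead, plays laser animations and drains Blackboard-held health through Timeline-driven damage, teleporting the player at zero.
; SetHealth4 then briefly shows CaughtUi and restores health.
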(event OnSeePawn(PawnSensing)
  (params (Pawn :type Pawn%20Object%20Reference))
  (bind _returnvalue (Utilities|Name|MakeLiteralName "IsPlayerRobotRange4"))
  (bind _self self)
  (bind _returnvalue_2 (AI|GetAIController _self))
  (bind _returnvalue_3 (AI|GetBlackboard _returnvalue_2))
  (Utilities|Casting|CastToBP_FirstPersonCharacter Pawn)
  (AI|Components|Blackboard|SetValueasBool _returnvalue_3 (Utilities|Name|MakeLiteralName "HasSeenPlayer4") true)
  (if (< (Transformation|GetDistanceTo Pawn (Game|GetPlayerCharacter 0)) (Variables|Default|GetRobotRange))
    (AI|Components|Blackboard|SetValueasBool _returnvalue_3 _returnvalue true)
    (else
      (AI|Components|Blackboard|SetValueasBool _returnvalue_3 _returnvalue false))))

(event Custom|SetHealth4
  (if (== (Class|BlackboardComponent|GetValueasFloat (AI|GetBlackboard (AI|GetAIController self)) (Utilities|Name|MakeLiteralName "CurrentHealth4")) 0.0)
    (bind _returnvalue (UserInterface|CreateWidget "/Game/UI/CaughtUi.CaughtUi_C"))
    (UserInterface|Viewport|AddtoViewport _returnvalue 0)
    (Utilities|FlowControl|Delay 2.0)
    (Widget|RemovefromParent _returnvalue)
    (AI|Components|Blackboard|SetValueasFloat (AI|GetBlackboard (AI|GetAIController self)) (Utilities|Name|MakeLiteralName "CurrentHealth4") 1.0)))

(event Custom|AttackPlayer4
  (bind _returnvalue (Transformation|GetActorLocation))
  (bind _returnvalue_2 (Utilities|Name|MakeLiteralName "CurrentHealth4"))
  (bind _self self)
  (bind _laser (Variables|Default|GetLaser))
  (bind _mesh (Variables|Character|GetMesh))
  (bind _returnvalue_3 (AI|GetAIController _self))
  (bind _returnvalue_4 (AI|GetBlackboard _returnvalue_3))
  (bind (_outhit _returnvalue_5) (Collision|SphereTraceForObjects _returnvalue (+ _returnvalue (* (Math|Vector|GetForwardVector (Transformation|GetActorRotation)) 2.5e+02)) 0.0 (Utilities|Array|MakeArray "ObjectTypeQuery3") false 0 "ForDuration"))
  (if _returnvalue_5
    (bind _asbp_first_person_character (Utilities|Casting|CastToBP_FirstPersonCharacter (.HitActor (Collision|BreakHitResult _outhit))))
    (Components|Animation|PlayAnimation _mesh "/Game/Animations/Robot/Roboco_skeletal_ANIMAZIONE_corrected_Anim.Roboco_skeletal_ANIMAZIONE_corrected_Anim" true)
    (Components|Animation|PlayAnimation _laser "/Game/Animations/Laser/Roboco_skeletal_ANIMAZIONE_Laser_Anim.Roboco_skeletal_ANIMAZIONE_Laser_Anim" true)
    (Rendering|Material|SetMaterial (Variables|Default|GetLaser) 0 "/Game/AI/Robot/Laser_2.Laser_2")
    (bind _range (Timeline|Timeline Play)
      (:Update
        (bind _returnvalue_6 (Game|Damage|ApplyDamage _asbp_first_person_character _range 0 _self))
        (AI|Components|Blackboard|SetValueasFloat _returnvalue_4 _returnvalue_2 (Math|Float|Clamp(Float) (- (Class|BlackboardComponent|GetValueasFloat _returnvalue_4 _returnvalue_2) _returnvalue_6) 0.0 (Variables|Default|GetMaxHealth)))
        (if (== (Math|Float|Clamp(Float) (- (Class|BlackboardComponent|GetValueasFloat _returnvalue_4 _returnvalue_2) _returnvalue_6) 0.0 (Variables|Default|GetMaxHealth)) 0.0)
          (Transformation|SetActorLocation _asbp_first_person_character (Math|Vector|MakeVector 1345.0 459.999917 1e+02) false false)
          (Pawn|SetControlRotation (Pawn|GetController _asbp_first_person_character) (Math|Rotator|MakeRotator 0.0 0.0 0.0))
          (AI|Components|Blackboard|SetValueasBool (AI|GetBlackboard (AI|GetAIController self)) (Utilities|Name|MakeLiteralName "IsPlayerRobotRange4") false)
          (AI|Components|Blackboard|SetValueasBool (AI|GetBlackboard (AI|GetAIController self)) (Utilities|Name|MakeLiteralName "HasSeenPlayer4") false)
          (Rendering|Material|SetMaterial (Variables|Default|GetLaser) 0 "/Game/AI/Robot/Laser.Laser")
          (Audio|Components|Audio|Stop _mesh)
          (Audio|Components|Audio|Stop _laser)
          (Timeline|Timeline Reverse))))))

(event EventBeginPlay
  (AI|Components|Blackboard|SetValueasFloat (AI|GetBlackboard (AI|GetAIController self)) (Utilities|Name|MakeLiteralName "CurrentHealth4") 1.0))

(fn ConstructionScript)

(fn GetPickupItemData
  (return 0))