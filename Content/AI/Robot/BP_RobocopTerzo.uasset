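; AI robot enemy that spots the first-person player and attacks with an animated laser.
; Pawn sensing sets seen and range blackboard keys, while AttackPlayer3 sphere-traces ahead and runs a damage timeline that drains the player health stored in CurrentHealth3.
; At zero health it teleports the player to a fixed point, clears the keys and stops the laser.
; CustomEvent_1 and CustomEvent_2 duplicate the attack and health reset for the "2" keys.
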(event OnSeePawn(PawnSensing)
  (params (Pawn :type Pawn%20Object%20Reference))
  (bind _returnvalue (Utilities|Name|MakeLiteralName "IsPlayerRobotRange3"))
  (bind _self self)
  (bind _returnvalue_2 (AI|GetAIController _self))
  (bind _returnvalue_3 (AI|GetBlackboard _returnvalue_2))
  (Utilities|Casting|CastToBP_FirstPersonCharacter Pawn)
  (AI|Components|Blackboard|SetValueasBool _returnvalue_3 (Utilities|Name|MakeLiteralName "HasSeenPlayer3") true)
  (if (< (Transformation|GetDistanceTo Pawn (Game|GetPlayerCharacter 0)) (Variables|Default|GetRobotRange))
    (AI|Components|Blackboard|SetValueasBool _returnvalue_3 _returnvalue true)
    (else
      (AI|Components|Blackboard|SetValueasBool _returnvalue_3 _returnvalue false))))

(event Custom|CustomEvent_2
  (AI|Components|Blackboard|SetValueasFloat (AI|GetBlackboard (AI|GetAIController self)) (Utilities|Name|MakeLiteralName "CurrentHealth2") 1.0))

(event Custom|AttackPlayer3
  (bind _returnvalue (Transformation|GetActorLocation))
  (bind _returnvalue_2 (Utilities|Name|MakeLiteralName "CurrentHealth3"))
  (bind _self self)
  (bind _mesh (Variables|Character|GetMesh))
  (bind _laser (Variables|Default|GetLaser))
  (bind _returnvalue_3 (AI|GetAIController _self))
  (bind _returnvalue_4 (AI|GetBlackboard _returnvalue_3))
  (bind (_outhit _returnvalue_5) (Collision|SphereTraceForObjects _returnvalue (+ _returnvalue (* (Math|Vector|GetForwardVector (Transformation|GetActorRotation)) 2.5e+02)) 0.0 (Utilities|Array|MakeArray "ObjectTypeQuery3") false 0 "ForDuration"))
  (if _returnvalue_5
    (bind _asbp_first_person_character (Utilities|Casting|CastToBP_FirstPersonCharacter (.HitActor (Collision|BreakHitResult _outhit))))
    (Components|Animation|PlayAnimation _mesh "/Game/Animations/Robot/Roboco_skeletal_ANIMAZIONE_corrected_Anim.Roboco_skeletal_ANIMAZIONE_corrected_Anim" true)
    (Components|Animation|PlayAnimation _laser "/Game/Animations/Laser/Roboco_skeletal_ANIMAZIONE_Laser_Anim.Roboco_skeletal_ANIMAZIONE_Laser_Anim" true)
    (Rendering|Material|SetMaterial (Variables|Default|GetLaser) 0 "/Game/AI/Robot/Laser_2.Laser_2")
    (bind _newtrack_0 (Timeline|Timeline Play)
      (:Update
        (bind _returnvalue_6 (Game|Damage|ApplyDamage _asbp_first_person_character _newtrack_0 0 _self))
        (Development|PrintString (Utilities|String|ToString(Float) (Math|Float|Clamp(Float) (- (Class|BlackboardComponent|GetValueasFloat _returnvalue_4 _returnvalue_2) _returnvalue_6) 0.0 (Variables|Default|GetMaxHealth))))
        (AI|Components|Blackboard|SetValueasFloat _returnvalue_4 _returnvalue_2 (Math|Float|Clamp(Float) (- (Class|BlackboardComponent|GetValueasFloat _returnvalue_4 _returnvalue_2) _returnvalue_6) 0.0 (Variables|Default|GetMaxHealth)))
        (if (== (Math|Float|Clamp(Float) (- (Class|BlackboardComponent|GetValueasFloat _returnvalue_4 _returnvalue_2) _returnvalue_6) 0.0 (Variables|Default|GetMaxHealth)) 0.0)
          (Transformation|SetActorLocation _asbp_first_person_character (Math|Vector|MakeVector 712.0 2731.0 100.917499) false false)
          (Pawn|SetControlRotation (Pawn|GetController _asbp_first_person_character) (Math|Rotator|MakeRotator 0.0 0.0 0.0))
          (AI|Components|Blackboard|SetValueasBool (AI|GetBlackboard (AI|GetAIController self)) (Utilities|Name|MakeLiteralName "IsPlayerRobotRange3") false)
          (AI|Components|Blackboard|SetValueasBool (AI|GetBlackboard (AI|GetAIController self)) (Utilities|Name|MakeLiteralName "HasSeenPlayer3") false)
          (Rendering|Material|SetMaterial (Variables|Default|GetLaser) 0 "/Game/AI/Robot/Laser.Laser")
          (Audio|Components|Audio|Stop _mesh)
          (Audio|Components|Audio|Stop _laser)
          (Timeline|Timeline Reverse))))))

(event Custom|CustomEvent_1
  (bind _returnvalue (Transformation|GetActorLocation))
  (bind _returnvalue_2 (Utilities|Name|MakeLiteralName "CurrentHealth2"))
  (bind _self self)
  (bind _laser (Variables|Default|GetLaser))
  (bind _mesh (Variables|Character|GetMesh))
  (bind _returnvalue_3 (AI|GetAIController _self))
  (bind _returnvalue_4 (AI|GetBlackboard _returnvalue_3))
  (bind (_outhit _returnvalue_5) (Collision|SphereTraceForObjects _returnvalue (+ _returnvalue (* (Math|Vector|GetForwardVector (Transformation|GetActorRotation)) 2.5e+02)) 0.0 (Utilities|Array|MakeArray "ObjectTypeQuery3") false 0 "ForDuration"))
  (if _returnvalue_5
    (bind _asbp_first_person_character (Utilities|Casting|CastToBP_FirstPersonCharacter (.HitActor (Collision|BreakHitResult _outhit))))
    (Components|Animation|PlayAnimation _mesh "/Game/Animations/Robot/Roboco_skeletal_ANIMAZIONE_corrected_Anim.Roboco_skeletal_ANIMAZIONE_corrected_Anim" true)
    (Components|Animation|PlayAnimation _laser "/Game/Animations/Laser/Roboco_skeletal_ANIMAZIONE_Laser_Anim.Roboco_skeletal_ANIMAZIONE_Laser_Anim" true)
    (Rendering|Material|SetMaterial (Variables|Default|GetLaser) 0 "/Game/AI/Robot/Laser_2.Laser_2")
    (bind _newtrack_0 (Timeline|Timeline_0 Play)
      (:Update
        (bind _returnvalue_6 (Game|Damage|ApplyDamage _asbp_first_person_character _newtrack_0 0 _self))
        (Development|PrintString (Utilities|String|ToString(Float) (Math|Float|Clamp(Float) (- (Class|BlackboardComponent|GetValueasFloat _returnvalue_4 _returnvalue_2) _returnvalue_6) 0.0 (Variables|Default|GetMaxHealth))))
        (AI|Components|Blackboard|SetValueasFloat _returnvalue_4 _returnvalue_2 (Math|Float|Clamp(Float) (- (Class|BlackboardComponent|GetValueasFloat _returnvalue_4 _returnvalue_2) _returnvalue_6) 0.0 (Variables|Default|GetMaxHealth)))
        (if (== (Math|Float|Clamp(Float) (- (Class|BlackboardComponent|GetValueasFloat _returnvalue_4 _returnvalue_2) _returnvalue_6) 0.0 (Variables|Default|GetMaxHealth)) 0.0)
          (Transformation|SetActorLocation _asbp_first_person_character (Math|Vector|MakeVector 712.0 2731.0 100.917499) false false)
          (Pawn|SetControlRotation (Pawn|GetController _asbp_first_person_character) (Math|Rotator|MakeRotator 0.0 0.0 0.0))
          (AI|Components|Blackboard|SetValueasBool (AI|GetBlackboard (AI|GetAIController self)) (Utilities|Name|MakeLiteralName "IsPlayerRobotRange2") false)
          (AI|Components|Blackboard|SetValueasBool (AI|GetBlackboard (AI|GetAIController self)) (Utilities|Name|MakeLiteralName "HasSeenPlayer2") false)
          (Rendering|Material|SetMaterial (Variables|Default|GetLaser) 0 "/Game/AI/Robot/Laser.Laser")
          (Audio|Components|Audio|Stop _mesh)
          (Audio|Components|Audio|Stop _laser)
          (Timeline|Timeline_0 Reverse))))))

(event Custom|SetHealth3
  (AI|Components|Blackboard|SetValueasFloat (AI|GetBlackboard (AI|GetAIController self)) (Utilities|Name|MakeLiteralName "CurrentHealth3") 1.0))

(fn ConstructionScript)