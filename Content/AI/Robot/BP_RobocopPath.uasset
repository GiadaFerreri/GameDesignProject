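; Robocop AI enemy that spots a visible player, immobilizes them with a laser and sends them back when caught.
; PawnSensing sets blackboard flags for sighting and range.
; AttackPlayer sphere-traces ahead, then a Timeline applies damage and drains CurrentHealth on the robot's blackboard.
; At zero it shows the caught widget, teleports both to hardcoded positions and clears the flags; BuGRobot offers a delayed robot-only reset.
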(event OnSeePawn(PawnSensing)
  (params (Pawn :type Pawn%20Object%20Reference))
  (bind _returnvalue (Utilities|Name|MakeLiteralName "IsPlayerRobotInRange"))
  (bind _self self)
  (bind _returnvalue_2 (AI|GetAIController _self))
  (bind _returnvalue_3 (AI|GetBlackboard _returnvalue_2))
  (bind _asbp_first_person_character (Utilities|Casting|CastToBP_FirstPersonCharacter Pawn))
  (if (Variables|/Game/FirstPerson/Blueprints/BP_FirstPersonCharacter.BP_FirstPersonCharacter_C|GetVisible? _asbp_first_person_character)
    (AI|Components|Blackboard|SetValueasBool _returnvalue_3 (Utilities|Name|MakeLiteralName "HasSeenPlayer") true)
    (if (< (Transformation|GetDistanceTo Pawn (Game|GetPlayerCharacter 0)) (Variables|Default|GetRobotRange))
      (AI|Components|Blackboard|SetValueasBool _returnvalue_3 _returnvalue true)
      (else
        (AI|Components|Blackboard|SetValueasBool _returnvalue_3 _returnvalue false)))))

(event Custom|Attack%20Player
  (bind _returnvalue (Transformation|GetActorLocation))
  (bind _returnvalue_2 (Utilities|Name|MakeLiteralName "CurrentHealth"))
  (bind _self self)
  (bind _self_2 self)
  (bind _laser (Variables|Default|GetLaser))
  (bind _mesh (Variables|Character|GetMesh))
  (bind _returnvalue_3 (AI|GetAIController _self))
  (bind _returnvalue_4 (AI|GetBlackboard _returnvalue_3))
  (bind (_outhit _returnvalue_5) (Collision|SphereTraceForObjects _returnvalue (+ _returnvalue (* (Math|Vector|GetForwardVector (Transformation|GetActorRotation)) 2.5e+02)) 0.0 (Utilities|Array|MakeArray "ObjectTypeQuery3") false 0 "ForDuration" true "(R=0.000000,G=0.000000,B=0.000000,A=0.000000)" "(R=0.000000,G=0.000000,B=0.000000,A=0.000000)" 1.0))
  (if _returnvalue_5
    (bind _asbp_first_person_character (Utilities|Casting|CastToBP_FirstPersonCharacter (.HitActor (Collision|BreakHitResult _outhit))))
    (Components|Animation|PlayAnimation _mesh "/Game/Animations/Robot/Roboco_skeletal_ANIMAZIONE_corrected_Anim.Roboco_skeletal_ANIMAZIONE_corrected_Anim" true)
    (Components|Animation|PlayAnimation _laser "/Game/Animations/Laser/Roboco_skeletal_ANIMAZIONE_Laser_Anim.Roboco_skeletal_ANIMAZIONE_Laser_Anim" true)
    (Rendering|Material|SetMaterial (Variables|Default|GetLaser) 0 "/Game/AI/Robot/Laser_2.Laser_2")
    (Pawn|Components|CharacterMovement|DisableMovement (Variables|/Script/Engine.Character|GetCharacterMovement _asbp_first_person_character))
    (bind _range (Timeline|Timeline Play)
      (:Update
        (bind _returnvalue_6 (Game|Damage|ApplyDamage _asbp_first_person_character _range 0 _self))
        (AI|Components|Blackboard|SetValueasFloat _returnvalue_4 _returnvalue_2 (Math|Float|Clamp(Float) (- (Class|BlackboardComponent|GetValueasFloat _returnvalue_4 _returnvalue_2) _returnvalue_6) 0.0 (Variables|Default|GetMaxHealth)))
        (if (== (Math|Float|Clamp(Float) (- (Class|BlackboardComponent|GetValueasFloat _returnvalue_4 _returnvalue_2) _returnvalue_6) 0.0 (Variables|Default|GetMaxHealth)) 0.0)
          (CallFunction|Dead)
          (Pawn|Components|CharacterMovement|SetMovementMode (Variables|/Script/Engine.Character|GetCharacterMovement _asbp_first_person_character) "MOVE_Walking" 0)
          (Transformation|SetActorLocation _asbp_first_person_character (Math|Vector|MakeVector 1345.0 459.999917 1e+02) false false)
          (Pawn|SetControlRotation (Pawn|GetController _asbp_first_person_character) (Math|Rotator|MakeRotator 0.0 0.0 0.0))
          (Transformation|SetActorLocation _self_2 (Math|Vector|MakeVector 3622.0 934.0 86.0) false false)
          (AI|Components|Blackboard|SetValueasBool (AI|GetBlackboard (AI|GetAIController _self_2)) (Utilities|Name|MakeLiteralName "IsPlayerRobotInRange") false)
          (AI|Components|Blackboard|SetValueasBool (AI|GetBlackboard (AI|GetAIController self)) (Utilities|Name|MakeLiteralName "HasSeenPlayer") false)
          (Rendering|Material|SetMaterial (Variables|Default|GetLaser) 0 "/Game/AI/Robot/Laser.Laser")
          (Audio|Components|Audio|Stop _mesh)
          (Audio|Components|Audio|Stop _laser)
          (Timeline|Timeline Reverse))))))

(event Custom|SetHealth
  (AI|Components|Blackboard|SetValueasFloat (AI|GetBlackboard (AI|GetAIController self)) (Utilities|Name|MakeLiteralName "CurrentHealth") 1.0))

(event Custom|Dead
  (Utilities|FlowControl|DoOnce false :!label _label
    (:Completed
      (bind _returnvalue (UserInterface|CreateWidget "/Game/UI/CaughtUi.CaughtUi_C" (Game|GetPlayerController 0)))
      (bind _output_get (Variables|Default|SetCaughtUi _returnvalue))
      (UserInterface|Viewport|AddtoViewport _output_get 0)
      (Utilities|FlowControl|Delay 2.0)
      (Widget|RemovefromParent _output_get)
      (goto _label Reset))))

(event Custom|BuGRobot
  (bind _self self)
  (bind _returnvalue (AI|GetAIController _self))
  (bind _returnvalue_2 (AI|GetBlackboard _returnvalue))
  (Utilities|FlowControl|Delay 3.0)
  (Transformation|SetActorLocation _self (Math|Vector|MakeVector 3622.0 934.0 86.0) false false)
  (AI|Components|Blackboard|SetValueasBool _returnvalue_2 (Utilities|Name|MakeLiteralName "IsPlayerRobotInRange") false)
  (AI|Components|Blackboard|SetValueasBool _returnvalue_2 (Utilities|Name|MakeLiteralName "HasSeenPlayer") false))

(fn ConstructionScript)

(fn GetPickupItemData
  (return 0))