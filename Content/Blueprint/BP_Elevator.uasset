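; BP_Elevator is an elevator whose two doors move when the player interacts with it, provided the player character has the map.
; The interaction plays a 2D elevator sound and starts a Timeline that drives each door's relative X position from its own track.
; A short Delay chained to the Timeline's Update, rather than to Finished, then reverses the Timeline to send the doors back.
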(event EventOnInteraction
  (params (playercharacter :type BP%20First%20Person%20Character%20Object%20Reference))
  (if (Variables|/Game/FirstPerson/Blueprints/BP_FirstPersonCharacter.BP_FirstPersonCharacter_C|GetHasMap playercharacter)
    (Audio|PlaySound2D "/Game/AUDIO/ASCENSORE.ASCENSORE" 1.0 1.0 0.0 0 0)
    (bind (_direction _newtrack_0 _seconda) (Timeline|Timeline Play)
      (:Update
        (Transformation|SetRelativeLocation (Variables|Default|GetElevatorDoor2) (Math|Vector|MakeVector _newtrack_0 0.0 0.0) false false)
        (Transformation|SetRelativeLocation (Variables|Default|GetElevatorDoor1) (Math|Vector|MakeVector _seconda 0.0 0.0) false false)
        (Utilities|FlowControl|Delay 3.5)
        (Timeline|Timeline Reverse)))))

(fn ConstructionScript)