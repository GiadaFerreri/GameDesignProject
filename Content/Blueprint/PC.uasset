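; Interactable PC that lets a player carrying the chiavetta (USB stick) run a timed download to obtain HasChiavettaIncredibile.
; Interaction resets HasTaken and shows the mission widget, then, if HasChiavetta, plays a sound and drives a progress bar from a timeline.
; HasTaken becoming true mid-download stops the timeline and removes the bar.
; Completion sets the flag, clears both widgets, briefly shows a success message, then adds a follow-up widget.
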(event EventOnInteraction
  (params (playercharacter :type BP%20First%20Person%20Character%20Object%20Reference))
  (Variables|/Game/FirstPerson/Blueprints/BP_FirstPersonCharacter.BP_FirstPersonCharacter_C|SetHasTaken? playercharacter false)
  (bind _returnvalue (UserInterface|CreateWidget "/Game/UI/Mission/MissionChiavetta.MissionChiavetta_C"))
  (UserInterface|Viewport|AddtoViewport _returnvalue 0)
  (if (Variables|/Game/FirstPerson/Blueprints/BP_FirstPersonCharacter.BP_FirstPersonCharacter_C|GetHasChiavetta? playercharacter)
    (Audio|PlaySound2D "/Game/AUDIO/SOUND_DOWNLOAD.SOUND_DOWNLOAD" 1.0 1.0 0.0 0 0)
    (bind _returnvalue_2 (UserInterface|CreateWidget "/Game/UI/BarradiCaricamento.BarradiCaricamento_C"))
    (bind _output_get (Variables|Default|Setbarra _returnvalue_2))
    (UserInterface|Viewport|AddtoViewport _output_get 0)
    (bind _track1 (Timeline|Progress PlayFromStart)
      (:Update
        (Progress|SetPercent (Variables|/Game/UI/BarradiCaricamento.BarradiCaricamento_C|GetProgressBar_0 (Variables|Default|Getbarra)) _track1)
        (if (Variables|/Game/FirstPerson/Blueprints/BP_FirstPersonCharacter.BP_FirstPersonCharacter_C|GetHasTaken? playercharacter)
          (Utilities|FlowControl|Sequence
            (:then_0
              (Timeline|Progress Stop))
            (:then_1
              (Widget|RemovefromParent _output_get)))))
      (:Finished
        (Variables|/Game/FirstPerson/Blueprints/BP_FirstPersonCharacter.BP_FirstPersonCharacter_C|SetHasChiavettaIncredibile? playercharacter true)
        (Widget|RemovefromParent _output_get)
        (Widget|RemovefromParent _returnvalue)
        (bind _returnvalue_3 (UserInterface|CreateWidget "/Game/UI/Caricamentoriuscito.Caricamentoriuscito_C"))
        (UserInterface|Viewport|AddtoViewport _returnvalue_3 0)
        (Utilities|FlowControl|Delay 3.0)
        (Widget|RemovefromParent _returnvalue_3)
        (bind _returnvalue_4 (UserInterface|CreateWidget "/Game/UI/Mission/MadreFiglio.MadreFiglio_C"))
        (UserInterface|Viewport|AddtoViewport _returnvalue_4 0)))))

(fn ConstructionScript)