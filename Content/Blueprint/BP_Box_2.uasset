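; BP_Box_2 is an interactable box that plays a chest-opening sound on interaction and animates only if the player character has a badge.
; Timeline_0 slides the box component (Scatola) along its relative X axis.
; Each update of that slide also triggers a FlipFlop, alternately playing and reversing a second timeline that drives the pitch of the lid (Coperchio).
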(event EventOnInteraction
  (params (playercharacter :type BP%20First%20Person%20Character%20Object%20Reference))
  (Audio|PlaySound2D "/Game/AUDIO/OPEN_CHEST.OPEN_CHEST" 1.0 1.0 0.0 0 0)
  (if (Variables|/Game/FirstPerson/Blueprints/BP_FirstPersonCharacter.BP_FirstPersonCharacter_C|GetHasBadge? playercharacter)
    (bind _location (Timeline|Timeline_0 Play)
      (:Update
        (Transformation|SetRelativeLocation (Variables|Default|GetScatola) (Math|Vector|MakeVector _location 0.0 0.0) false false)
        (Utilities|FlowControl|FlipFlop
          (:A
            (bind _newtrack_0 (Timeline|Timeline Play)
              (:Update
                (Transformation|SetRelativeRotation (Variables|Default|GetCoperchio) (Math|Rotator|MakeRotator 0.0 _newtrack_0 0.0) false false))))
          (:B
            (Timeline|Timeline Reverse)))))))

(fn ConstructionScript)